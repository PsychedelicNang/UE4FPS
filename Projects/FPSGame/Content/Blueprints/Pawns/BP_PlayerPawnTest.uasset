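; BP_PlayerPawnTest is a player pawn Blueprint with debug keys for exercising its health component.
; H heals a fixed amount and K calls KillSelf to test the death animation.
; ForwardTrace line-traces from the camera along its forward vector on the Visibility channel, with debug drawing, and returns the hit.
; Crosshair and HUD widget creation nodes exist but are disconnected, and BeginPlay is empty.
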(event `self.ReceiveBeginPlay`)

(event `Key|H`
  (params (Key :type "Key Structure"))
  ;[1 1 1] Test healing
  (:`Pressed`
    (`ShooterHealthComponent.Heal` (`self.HealthComp`) 20.0)))

(event `Key|K`
  (params (Key :type "Key Structure"))
  ;[1 1 1] Test death animation
  (:`Pressed`
    (`ShooterHealthComponent.KillSelf` (`self.HealthComp`))))

(fn `ForwardTrace`
  (params (Distance :type "Float (double-precision)"))
  (returns (OutHit :type "HitResult Structure") (HitAnything :type Boolean))
  (bind _cameracomp (`self.CameraComp`))
  (bind _returnvalue (`SceneComponent.K2_GetComponentLocation` _cameracomp))
  (bind (_outhit _returnvalue_2) (`KismetSystemLibrary.LineTraceSingle` :`Start` _returnvalue :`End` (+ _returnvalue (* (`SceneComponent.GetForwardVector` _cameracomp) Distance)) :`TraceChannel` "TraceTypeQuery1" :`DrawDebugType` "ForDuration"))
  (return _outhit _returnvalue_2))

(fn `UserConstructionScript`)